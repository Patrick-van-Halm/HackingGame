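; BP_Player is a player Blueprint that drives a custom on-screen cursor with mouse input.
; On BeginPlay it creates the BP_ScreenInterface widget and adds it to the player screen.
; MouseX and MouseY share one path that scales an axis value by base plus additional speeds, inverts Y, and adds it to the stored position.
; UpdateCurserPos saves that position and moves the cursor image's canvas slot, without clamping.
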(event `self.ReceiveBeginPlay`
  (bind _returnvalue (`|CreateWidget` "/Game/Blueprints/BP_ScreenInterface.BP_ScreenInterface_C"))
  (bind _output_get (set `self.ScreenUI` _returnvalue))
  (`UserWidget.AddToPlayerScreen` _output_get 0))

(event `InputAxisKey|MouseX`
  (params (AxisValue :type "Float (single-precision)"))
  (`self.UpdateCurserPos` (+ (`KismetMathLibrary.MakeVector2D` (* AxisValue (+ (`self.CursorBaseSpeedX`) (`self.CursorSpeedX`))) (* (stale `InputAxisKey|MouseY` AxisValue) (+ (`self.CursorBaseSpeedY`) (`self.CursorSpeedY`)) -1.0)) (`self.CurCursorPos`)) :!label _label))

(event `InputAxisKey|MouseY`
  (params (AxisValue :type "Float (single-precision)"))
  (goto _label))

(fn `UpdateCurserPos`
  (params (NewPos :type "Vector2D Structure"))
  (bind _output_get (set `self.CurCursorPos` NewPos))
  (`CanvasPanelSlot.SetPosition` (`WidgetLayoutLibrary.SlotAsCanvasSlot` (`/Game/Blueprints/BP_ScreenInterface.IMG_Curser` (`self.ScreenUI`))) _output_get))

(fn `UserConstructionScript`)